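; BP_Pumps is a pump prop actor with a configurable number decal and fill level.
; The construction script calls ChangeNumber, which assigns the DecalNumber mesh to two trim decal components.
; It then calls WaterLevel, which passes FillLevel to the FillHeight scalar parameter on the pump mesh's materials.
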(event Custom|ChangeNumber
  (bind _decalnumber (Variables|Default|GetDecalNumber))
  (Components|StaticMesh|SetStaticMesh (Variables|Default|GetDecalNumbers_Trim_Chiffre021) _decalnumber)
  (Components|StaticMesh|SetStaticMesh (Variables|Default|GetDecalNumbers_Trim_Chiffre022) _decalnumber))

(event Custom|WaterLevel
  (Rendering|Material|SetScalarParameterValueonMaterials (Variables|Default|GetSM_Pump) "FillHeight" (Variables|Default|GetFillLevel)))

(fn ConstructionScript
  (CallFunction|ChangeNumber)
  (CallFunction|WaterLevel))