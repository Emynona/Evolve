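; Point light actor Blueprint that produces a short, triggered flash of light.
; The light starts hidden on BeginPlay.
; The Lumiere event shows it, then hides it again after a half-second delay.
; The Detruit event hides it immediately, without cancelling any pending delay.
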(event Custom|Lumiere
  (Rendering|SetVisibility (Variables|Default|GetPointLightComponent) true false)
  (Utilities|FlowControl|Delay 0.5)
  (Rendering|SetVisibility (Variables|Default|GetLightComponent) false false))

(event Custom|Detruit
  (Rendering|SetVisibility (Variables|Default|GetPointLightComponent) false false))

(event EventBeginPlay
  (Rendering|SetVisibility (Variables|Default|GetPointLightComponent) false false))

(fn ConstructionScript)