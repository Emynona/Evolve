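; BP_Pumps01 is a destructible pump prop with a configurable decal number and visible fill level.
; The construction script applies the number mesh to both decals and drives the pump material's FillHeight parameter from FillLevel.
; Dégats plays a metallic impact sound; Destruction hides the pump and decals, spawns explosion and smoke Niagara effects at the Arrow, plays a destruction sound, and swaps the running audio for the inactivity loop.
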(event Custom|ChangeNumber
  (bind _decalnumber (Variables|Default|GetDecalNumber))
  (Components|StaticMesh|SetStaticMesh (Variables|Default|GetDecalNumbers_Trim_Chiffre021) _decalnumber)
  (Components|StaticMesh|SetStaticMesh (Variables|Default|GetDecalNumbers_Trim_Chiffre022) _decalnumber))

(event Custom|WaterLevel
  (Rendering|Material|SetScalarParameterValueonMaterials (Variables|Default|GetSM_Pump) "FillHeight" (Variables|Default|GetFillLevel)))

(event Custom|Destruction
  (bind _arrow (Variables|Default|GetArrow))
  (bind _pump_base (Variables|Default|GetPump_Base))
  (bind _returnvalue (Transformation|GetWorldTransform _arrow))
  (Audio|Components|Audio|Stop (Variables|Default|GetEvolve_FX_-_Pompes_Bruit_de_pompe_style_pompe_à_chaleur_Cue))
  (Niagara|SpawnSystemAttached "/Game/Evolve/Art/FX/Explosion/NS_Explosion.NS_Explosion" _pump_base "None" (.location _returnvalue) (.rotation _returnvalue) "KeepWorldPosition" false)
  (Rendering|SetVisibility (Variables|Default|GetSM_Pump) false false)
  (Niagara|SpawnSystemAttached "/Game/Evolve/Art/FX/Smoke/NS_Smoke.NS_Smoke" _pump_base "None" (.location _returnvalue) (.rotation _returnvalue) "KeepWorldPosition" false)
  (Audio|SpawnSoundAttached "/Game/Evolve/Art/Audios/Sons/Evolve_FX_-_Generateur_Bruit_de_destruction1_Cue.Evolve_FX_-_Generateur_Bruit_de_destruction1_Cue" _pump_base "None" (.location _returnvalue) (.rotation _returnvalue) "KeepWorldPosition" false 1e+01 1.0 1.5 0 0)
  (Audio|Components|Audio|Play (Variables|Default|GetEvolve_FX_-_Pompe_Bruit_d’inactivité_Cue) 0.0))

(event Custom|Dégats
  (bind _arrow (Variables|Default|GetArrow))
  (bind _returnvalue (Transformation|GetWorldTransform _arrow))
  (Audio|SpawnSoundAttached "/Game/Evolve/Art/Audios/Sons/Evolve_FX_-_Pompe_Bruit_impact_métallique_Cue.Evolve_FX_-_Pompe_Bruit_impact_métallique_Cue" (Variables|Default|GetPump_Base) "None" (.location _returnvalue) (.rotation _returnvalue) "KeepWorldPosition" false 0.75 1.0 0.0 0 0))

(event EventBeginPlay
  (Audio|Components|Audio|Stop (Variables|Default|GetEvolve_FX_-_Pompe_Bruit_d’inactivité_Cue)))

(fn ConstructionScript
  (CallFunction|ChangeNumber)
  (CallFunction|WaterLevel))