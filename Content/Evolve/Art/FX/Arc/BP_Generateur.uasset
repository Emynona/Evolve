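; BP_Generateur is a generator FX Blueprint that animates a Niagara component rising in a repeating loop.
; Each Tick, a helper function raises the component's relative Z by a fixed step, so speed depends on frame rate.
; When the new height exactly equals the CylinderHeight component's Z, the effect teleports back to a hardcoded start location; the equality test has no tolerance.
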(event EventTick
  (params (DeltaSeconds :type Float%20%28single-precision%29))
  (CallFunction|NewFunction0 0.5 (Variables|Default|GetNiagara)))

(fn ConstructionScript)

(fn NewFunction0
  (params (Speed :type Float%20%28single-precision%29) (Target :type Scene%20Component%20Object%20Reference))
  (bind _relativelocation (Variables|/Script/Engine.SceneComponent|GetRelativeLocation Target))
  (bind _returnvalue (+ (.z _relativelocation) Speed))
  (Transformation|SetRelativeLocation Target (Math|Vector|MakeVector (.x _relativelocation) (.y _relativelocation) _returnvalue) false false)
  (if (== _returnvalue (.z (Variables|/Script/Engine.SceneComponent|GetRelativeLocation (Variables|Default|GetCylinder_Height))))
    (Transformation|SetRelativeLocation (Variables|Default|GetNiagara) (Math|Vector|MakeVector -1.4e+02 0.0 0.0) false true)))