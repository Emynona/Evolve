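; Enemy wave spawner that registers with BP_GameMode and runs a five-wave countdown with per-wave UI banners.
; WaveSpawn starts a looping timer that spawns fixed enemy groups and increments the GameMode's enemy count until the wave quota runs out.
; Middle waves spawn only when certain GameMode Pompe flags are set, otherwise calling NextWave.
; Spawned waves end by triggering GameMode AI spawn or move events; a separate Win function pauses and shows UI_Win.
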(event Custom|Lancement
  ;[1 1 1] Spawn Dynamique Ennemies
  (bind _asbp_game_mode (Utilities|Casting|CastToBP_GameMode (Game|GetGameMode)))
  (bind _output_get (Variables|Default|SetBP_GameMode _asbp_game_mode))
  (Variables|/Game/Evolve/Core/GameMode/BP_GameMode.BP_GameMode_C|SetBP_Spawner _output_get self)
  (Variables|/Game/Evolve/Core/GameMode/BP_GameMode.BP_GameMode_C|SetNbWaveCurrent (Variables|Default|GetBP_GameMode) (Variables|Default|GetNbWaves))
  (Variables|Default|SetNbEnemiesCurrent (Variables|Default|GetNbEnemiesWave1))
  (CallFunction|WaveSpawn))

(event Custom|WaveSpawn
  ;[1 1 1] Spawn Dynamique Ennemies
  (Class|BPIMPGameMode|Cylindre(Message) (Variables|Default|GetBP_GameMode))
  (Utilities|FlowControl|Delay 2.0)
  (bind _result (Math|Integer|DecrementInt (Variables|/Game/Evolve/Core/GameMode/BP_GameMode.BP_GameMode_C|GetNbWaveCurrent (Variables|Default|GetBP_GameMode)))
    (:%20%20
      (if (>= _result 0)
        (bind _returnvalue (Utilities|Time|SetTimerbyEvent (delegate Custom|SpawnMechant) (Variables|Default|GetIntervalleBetweenSpawn) true))
        (Variables|Default|SetHandleTimer _returnvalue)
        (Utilities|FlowControl|DoOnce false
          (:Completed
            (bind _returnvalue_2 (UserInterface|CreateWidget "/Game/Evolve/UI/UI_Vague1.UI_Vague1_C"))
            (UserInterface|Viewport|AddtoViewport _returnvalue_2 0)
            (Variables|Default|SetWidgetRef _returnvalue_2)))))))

(event Custom|SpawnMechant
  (bind _bp_gamemode (Variables|Default|GetBP_GameMode))
  (bind _bp_gamemode_2 (Variables|Default|GetBP_GameMode))
  (bind _bp_gamemode_3 (Variables|Default|GetBP_GameMode))
  (bind _bp_gamemode_4 (Variables|Default|GetBP_GameMode))
  (bind _bp_gamemode_5 (Variables|Default|GetBP_GameMode))
  (bind _bp_gamemode_6 (Variables|Default|GetBP_GameMode))
  (bind _bp_gamemode_7 (Variables|Default|GetBP_GameMode))
  (bind _bp_gamemode_8 (Variables|Default|GetBP_GameMode))
  (bind _bp_gamemode_9 (Variables|Default|GetBP_GameMode))
  (bind _bp_gamemode_10 (Variables|Default|GetBP_GameMode))
  (bind _bp_gamemode_11 (Variables|Default|GetBP_GameMode))
  (bind _bp_gamemode_12 (Variables|Default|GetBP_GameMode))
  ;[1 1 1] Spawn Dynamique Ennemies
  (if (== (Variables|/Game/Evolve/Core/GameMode/BP_GameMode.BP_GameMode_C|GetNbWaveCurrent (Variables|Default|GetBP_GameMode)) 4)
    (Game|SpawnActorfromClass (Variables|Default|GetEnemy1) (Math|Transform|MakeTransform (Variables|Default|GetSpawn%20Transform%20Location) "0, 0, 0" "1,1,1") "Undefined" 0 0)
    (Math|Integer|IncrementInt (Variables|/Game/Evolve/Core/GameMode/BP_GameMode.BP_GameMode_C|GetNbEnnemies (Variables|Default|GetBP_GameMode))
      (:%20%20
        (Game|SpawnActorfromClass (Variables|Default|GetEnemy2) (Math|Transform|MakeTransform (Variables|Default|GetSpawn%20Transform%20Location_0) "0,90.000000, 0" "1,1,1") "Undefined" 0 0)
        (Math|Integer|IncrementInt (Variables|/Game/Evolve/Core/GameMode/BP_GameMode.BP_GameMode_C|GetNbEnnemies (Variables|Default|GetBP_GameMode))
          (:%20%20
            (Game|SpawnActorfromClass (Variables|Default|GetEnemy3) (Math|Transform|MakeTransform (Variables|Default|GetSpawn%20Transform%20Location_1) "0,90.000000, 0" "1,1,1") "Undefined" 0 0)
            (Math|Integer|IncrementInt (Variables|/Game/Evolve/Core/GameMode/BP_GameMode.BP_GameMode_C|GetNbEnnemies (Variables|Default|GetBP_GameMode))
              (:%20%20
                (Game|SpawnActorfromClass (Variables|Default|GetEnemy4) (Math|Transform|MakeTransform (Variables|Default|GetSpawn%20Transform%20Location_2) "0,90.000000, 0" "1,1,1") "Undefined" 0 0)
                (Math|Integer|IncrementInt (Variables|/Game/Evolve/Core/GameMode/BP_GameMode.BP_GameMode_C|GetNbEnnemies (Variables|Default|GetBP_GameMode))
                  (:%20%20
                    (Game|SpawnActorfromClass (Variables|Default|GetEnemy5) (Math|Transform|MakeTransform (Variables|Default|GetSpawn%20Transform%20Location_3) "0,90.000000, 0" "1,1,1") "Undefined" 0 0)
                    (Math|Integer|IncrementInt (Variables|/Game/Evolve/Core/GameMode/BP_GameMode.BP_GameMode_C|GetNbEnnemies (Variables|Default|GetBP_GameMode))
                      (:%20%20
                        (Game|SpawnActorfromClass (Variables|Default|GetEnemy6) (Math|Transform|MakeTransform (Variables|Default|GetSpawn%20Transform%20Location_4) "0,90.000000, 0" "1,1,1") "Undefined" 0 0)
                        (Math|Integer|IncrementInt (Variables|/Game/Evolve/Core/GameMode/BP_GameMode.BP_GameMode_C|GetNbEnnemies (Variables|Default|GetBP_GameMode))
                          (:%20%20
                            (bind _result (Math|Integer|DecrementInt (Variables|Default|GetNbEnemiesCurrent))
                              (:%20%20
                                (if (<= _result 0)
                                  (Variables|Default|SetNbEnemiesCurrent (Variables|Default|GetNbEnemiesWave2))
                                  (Utilities|Time|ClearandInvalidateTimerbyHandle (Variables|Default|GetHandleTimer))
                                  (Class|BPIMPGameMode|StopCylindre(Message) _bp_gamemode_6)
                                  (Variables|/Game/Evolve/Core/GameMode/BP_GameMode.BP_GameMode_C|SetP1 _bp_gamemode_6 true)
                                  (Default|SpawnIA1 _bp_gamemode_6)
                                  (Default|SpawnIA2 _bp_gamemode_6)
                                  (Default|SpawnIA3 _bp_gamemode_6)
                                  (Variables|/Game/Evolve/Core/GameMode/BP_GameMode.BP_GameMode_C|SetP1 _bp_gamemode_6 false)
                                  (Variables|/Game/Evolve/Core/GameMode/BP_GameMode.BP_GameMode_C|SetP2 _bp_gamemode_6 true)
                                  (Default|SpawnIA4 _bp_gamemode_6)
                                  (Default|SpawnIA5 _bp_gamemode_6)
                                  (Default|SpawnIA6 _bp_gamemode_6)
                                  (Variables|/Game/Evolve/Core/GameMode/BP_GameMode.BP_GameMode_C|SetP2 _bp_gamemode_6 false))))))))))))))))
    (else
      (Widget|RemovefromParent (Variables|Default|GetWidgetRef))
      (bind _returnvalue (UserInterface|CreateWidget "/Game/Evolve/UI/UI_Vague2.UI_Vague2_C"))
      (UserInterface|Viewport|AddtoViewport _returnvalue 0)
      (Variables|Default|SetWidgetRef _returnvalue)
      (if (== (Variables|/Game/Evolve/Core/GameMode/BP_GameMode.BP_GameMode_C|GetNbWaveCurrent _bp_gamemode_9) 3)
        (if (Variables|/Game/Evolve/Core/GameMode/BP_GameMode.BP_GameMode_C|GetPompe02 _bp_gamemode_9)
          (Game|SpawnActorfromClass (Variables|Default|GetEnemy1) (Math|Transform|MakeTransform (Variables|Default|GetSpawn%20Transform%20Location_5) "0,90.000000, 0" "1,1,1") "Undefined" 0 0 :!label _label)
          (Math|Integer|IncrementInt (Variables|/Game/Evolve/Core/GameMode/BP_GameMode.BP_GameMode_C|GetNbEnnemies (Variables|Default|GetBP_GameMode))
            (:%20%20
              (Game|SpawnActorfromClass (Variables|Default|GetEnemy3) (Math|Transform|MakeTransform (Variables|Default|GetSpawn%20Transform%20Location_6) "0,90.000000, 0" "1,1,1") "Undefined" 0 0)
              (Math|Integer|IncrementInt (Variables|/Game/Evolve/Core/GameMode/BP_GameMode.BP_GameMode_C|GetNbEnnemies (Variables|Default|GetBP_GameMode))
                (:%20%20
                  (Game|SpawnActorfromClass (Variables|Default|GetEnemy5) (Math|Transform|MakeTransform (Variables|Default|GetSpawn%20Transform%20Location_7) "0,90.000000, 0" "1,1,1") "Undefined" 0 0)
                  (Math|Integer|IncrementInt (Variables|/Game/Evolve/Core/GameMode/BP_GameMode.BP_GameMode_C|GetNbEnnemies (Variables|Default|GetBP_GameMode))
                    (:%20%20
                      (Game|SpawnActorfromClass (Variables|Default|GetEnemy6) (Math|Transform|MakeTransform (Variables|Default|GetSpawn%20Transform%20Location_8) "0,90.000000, 0" "1,1,1") "Undefined" 0 0)
                      (Math|Integer|IncrementInt (Variables|/Game/Evolve/Core/GameMode/BP_GameMode.BP_GameMode_C|GetNbEnnemies (Variables|Default|GetBP_GameMode))
                        (:%20%20
                          (bind _result_2 (Math|Integer|DecrementInt (Variables|Default|GetNbEnemiesCurrent))
                            (:%20%20
                              (if (<= _result_2 0)
                                (Variables|Default|SetNbEnemiesCurrent (Variables|Default|GetNbEnemiesWave3))
                                (Utilities|Time|ClearandInvalidateTimerbyHandle (Variables|Default|GetHandleTimer))
                                (Class|BPIMPGameMode|StopCylindre(Message) _bp_gamemode_2)
                                (Default|IasMoves _bp_gamemode_2))))))))))))
          (elif (Variables|/Game/Evolve/Core/GameMode/BP_GameMode.BP_GameMode_C|GetPompe01 _bp_gamemode_9)
            (goto _label)
            (elif (Variables|/Game/Evolve/Core/GameMode/BP_GameMode.BP_GameMode_C|GetPompe04 _bp_gamemode_9)
              (goto _label)
              (else
                (bind _result_3 (Math|Integer|DecrementInt (Variables|Default|GetNbEnemiesCurrent))
                  (:%20%20
                    (if (<= _result_3 0)
                      (Variables|Default|SetNbEnemiesCurrent (Variables|Default|GetNbEnemiesWave3))
                      (Utilities|Time|ClearandInvalidateTimerbyHandle (Variables|Default|GetHandleTimer))
                      (Class|BPIMPGameMode|StopCylindre(Message) _bp_gamemode_5)
                      (Default|NextWave _bp_gamemode_5))))))))
        (else
          (Widget|RemovefromParent (Variables|Default|GetWidgetRef))
          (bind _returnvalue_2 (UserInterface|CreateWidget "/Game/Evolve/UI/UI_Vague3.UI_Vague3_C"))
          (UserInterface|Viewport|AddtoViewport _returnvalue_2 0)
          (Variables|Default|SetWidgetRef _returnvalue_2)
          (if (== (Variables|/Game/Evolve/Core/GameMode/BP_GameMode.BP_GameMode_C|GetNbWaveCurrent _bp_gamemode) 2)
            (if (Variables|/Game/Evolve/Core/GameMode/BP_GameMode.BP_GameMode_C|GetPompe04 _bp_gamemode)
              (Game|SpawnActorfromClass (Variables|Default|GetEnemy1) (Math|Transform|MakeTransform (Variables|Default|GetSpawn%20Transform%20Location_9) "0,90.000000, 0" "1,1,1") "Undefined" 0 0 :!label _label_2)
              (Math|Integer|IncrementInt (Variables|/Game/Evolve/Core/GameMode/BP_GameMode.BP_GameMode_C|GetNbEnnemies (Variables|Default|GetBP_GameMode))
                (:%20%20
                  (Game|SpawnActorfromClass (Variables|Default|GetEnemy2) (Math|Transform|MakeTransform (Variables|Default|GetSpawn%20Transform%20Location_10) "0,90.000000, 0" "1,1,1") "Undefined" 0 0)
                  (Math|Integer|IncrementInt (Variables|/Game/Evolve/Core/GameMode/BP_GameMode.BP_GameMode_C|GetNbEnnemies (Variables|Default|GetBP_GameMode))
                    (:%20%20
                      (Game|SpawnActorfromClass (Variables|Default|GetEnemy3) (Math|Transform|MakeTransform (Variables|Default|GetSpawn%20Transform%20Location_11) "0,90.000000, 0" "1,1,1") "Undefined" 0 0)
                      (Math|Integer|IncrementInt (Variables|/Game/Evolve/Core/GameMode/BP_GameMode.BP_GameMode_C|GetNbEnnemies (Variables|Default|GetBP_GameMode))
                        (:%20%20
                          (Game|SpawnActorfromClass (Variables|Default|GetEnemy4) (Math|Transform|MakeTransform (Variables|Default|GetSpawn%20Transform%20Location_12) "0,90.000000, 0" "1,1,1") "Undefined" 0 0)
                          (Math|Integer|IncrementInt (Variables|/Game/Evolve/Core/GameMode/BP_GameMode.BP_GameMode_C|GetNbEnnemies (Variables|Default|GetBP_GameMode))
                            (:%20%20
                              (Game|SpawnActorfromClass (Variables|Default|GetEnemy5) (Math|Transform|MakeTransform (Variables|Default|GetSpawn%20Transform%20Location_13) "0,90.000000, 0" "1,1,1") "Undefined" 0 0)
                              (Math|Integer|IncrementInt (Variables|/Game/Evolve/Core/GameMode/BP_GameMode.BP_GameMode_C|GetNbEnnemies (Variables|Default|GetBP_GameMode))
                                (:%20%20
                                  (bind _result_4 (Math|Integer|DecrementInt (Variables|Default|GetNbEnemiesCurrent))
                                    (:%20%20
                                      (if (<= _result_4 0)
                                        (Variables|Default|SetNbEnemiesCurrent (Variables|Default|GetNbEnemiesWave4))
                                        (Utilities|Time|ClearandInvalidateTimerbyHandle (Variables|Default|GetHandleTimer))
                                        (Class|BPIMPGameMode|StopCylindre(Message) _bp_gamemode_7)
                                        (Default|IasMoves _bp_gamemode_7))))))))))))))
              (elif (Variables|/Game/Evolve/Core/GameMode/BP_GameMode.BP_GameMode_C|GetPompe03 _bp_gamemode)
                (goto _label_2)
                (elif (Variables|/Game/Evolve/Core/GameMode/BP_GameMode.BP_GameMode_C|GetPompe02 _bp_gamemode)
                  (Variables|Default|SetNbEnemiesCurrent (Variables|Default|GetNbEnemiesWave4))
                  (Utilities|Time|ClearandInvalidateTimerbyHandle (Variables|Default|GetHandleTimer))
                  (Class|BPIMPGameMode|StopCylindre(Message) _bp_gamemode_4)
                  (Default|NextWave _bp_gamemode_4)
                  (else
                    (Math|Integer|DecrementInt (Variables|/Game/Evolve/Core/GameMode/BP_GameMode.BP_GameMode_C|GetNbWaveCurrent (Variables|Default|GetBP_GameMode))
                      (:%20%20
                        (Variables|Default|SetNbEnemiesCurrent (Variables|Default|GetNbEnemiesWave5))
                        (Utilities|Time|ClearandInvalidateTimerbyHandle (Variables|Default|GetHandleTimer))
                        (Class|BPIMPGameMode|StopCylindre(Message) _bp_gamemode_3)
                        (Default|NextWave _bp_gamemode_3)))))))
            (else
              (Widget|RemovefromParent (Variables|Default|GetWidgetRef))
              (bind _returnvalue_3 (UserInterface|CreateWidget "/Game/Evolve/UI/UI_Vague4.UI_Vague4_C"))
              (UserInterface|Viewport|AddtoViewport _returnvalue_3 0)
              (Variables|Default|SetWidgetRef _returnvalue_3)
              (if (== (Variables|/Game/Evolve/Core/GameMode/BP_GameMode.BP_GameMode_C|GetNbWaveCurrent _bp_gamemode_10) 1)
                (if (Variables|/Game/Evolve/Core/GameMode/BP_GameMode.BP_GameMode_C|GetPompe02 _bp_gamemode_10)
                  (Game|SpawnActorfromClass (Variables|Default|GetEnemy1) (Math|Transform|MakeTransform (Variables|Default|GetSpawn%20Transform%20Location_14) "0,-90.000000, 0" "1,1,1") "Undefined" 0 0 :!label _label_3)
                  (Math|Integer|IncrementInt (Variables|/Game/Evolve/Core/GameMode/BP_GameMode.BP_GameMode_C|GetNbEnnemies (Variables|Default|GetBP_GameMode))
                    (:%20%20
                      (Game|SpawnActorfromClass (Variables|Default|GetEnemy2) (Math|Transform|MakeTransform (Variables|Default|GetSpawn%20Transform%20Location_15) "0,90.000000, 0" "1,1,1") "Undefined" 0 0)
                      (Math|Integer|IncrementInt (Variables|/Game/Evolve/Core/GameMode/BP_GameMode.BP_GameMode_C|GetNbEnnemies (Variables|Default|GetBP_GameMode))
                        (:%20%20
                          (Game|SpawnActorfromClass (Variables|Default|GetEnemy3) (Math|Transform|MakeTransform (Variables|Default|GetSpawn%20Transform%20Location_16) "0,90.000000, 0" "1,1,1") "Undefined" 0 0)
                          (Math|Integer|IncrementInt (Variables|/Game/Evolve/Core/GameMode/BP_GameMode.BP_GameMode_C|GetNbEnnemies (Variables|Default|GetBP_GameMode))
                            (:%20%20
                              (Game|SpawnActorfromClass (Variables|Default|GetEnemy4) (Math|Transform|MakeTransform (Variables|Default|GetSpawn%20Transform%20Location_17) "0,90.000000, 0" "1,1,1") "Undefined" 0 0)
                              (Math|Integer|IncrementInt (Variables|/Game/Evolve/Core/GameMode/BP_GameMode.BP_GameMode_C|GetNbEnnemies (Variables|Default|GetBP_GameMode))
                                (:%20%20
                                  (Game|SpawnActorfromClass (Variables|Default|GetEnemy6) (Math|Transform|MakeTransform (Variables|Default|GetSpawn%20Transform%20Location_18) "0,90.000000, 0" "1,1,1") "Undefined" 0 0)
                                  (Math|Integer|IncrementInt (Variables|/Game/Evolve/Core/GameMode/BP_GameMode.BP_GameMode_C|GetNbEnnemies (Variables|Default|GetBP_GameMode))
                                    (:%20%20
                                      (bind _result_5 (Math|Integer|DecrementInt (Variables|Default|GetNbEnemiesCurrent))
                                        (:%20%20
                                          (if (<= _result_5 0)
                                            (Variables|Default|SetNbEnemiesCurrent (Variables|Default|GetNbEnemiesWave5))
                                            (Utilities|Time|ClearandInvalidateTimerbyHandle (Variables|Default|GetHandleTimer))
                                            (Class|BPIMPGameMode|StopCylindre(Message) _bp_gamemode_11)
                                            (Default|IasMoves _bp_gamemode_11))))))))))))))
                  (elif (Variables|/Game/Evolve/Core/GameMode/BP_GameMode.BP_GameMode_C|GetPompe03 _bp_gamemode_10)
                    (goto _label_3)
                    (elif (Variables|/Game/Evolve/Core/GameMode/BP_GameMode.BP_GameMode_C|GetPompe04 _bp_gamemode_10)
                      (goto _label_3)
                      (else
                        (Variables|Default|SetNbEnemiesCurrent (Variables|Default|GetNbEnemiesWave5))
                        (Utilities|Time|ClearandInvalidateTimerbyHandle (Variables|Default|GetHandleTimer))
                        (Class|BPIMPGameMode|StopCylindre(Message) _bp_gamemode_8)
                        (Default|NextWave _bp_gamemode_8)))))
                (else
                  (Widget|RemovefromParent (Variables|Default|GetWidgetRef))
                  (bind _returnvalue_4 (UserInterface|CreateWidget "/Game/Evolve/UI/UI_Vague5.UI_Vague5_C"))
                  (UserInterface|Viewport|AddtoViewport _returnvalue_4 0)
                  (Variables|Default|SetWidgetRef _returnvalue_4)
                  (Game|SpawnActorfromClass (Variables|Default|GetEnemy1) (Math|Transform|MakeTransform (Variables|Default|GetSpawn%20Transform%20Location_19) "0,-90.000000,0.000000" "1,1,1") "Undefined" 0 0)
                  (Math|Integer|IncrementInt (Variables|/Game/Evolve/Core/GameMode/BP_GameMode.BP_GameMode_C|GetNbEnnemies (Variables|Default|GetBP_GameMode))
                    (:%20%20
                      (Game|SpawnActorfromClass (Variables|Default|GetEnemy2) (Math|Transform|MakeTransform (Variables|Default|GetSpawn%20Transform%20Location_20) "0,90.000000, 0" "1,1,1") "Undefined" 0 0)
                      (Math|Integer|IncrementInt (Variables|/Game/Evolve/Core/GameMode/BP_GameMode.BP_GameMode_C|GetNbEnnemies (Variables|Default|GetBP_GameMode))
                        (:%20%20
                          (Game|SpawnActorfromClass (Variables|Default|GetEnemy3) (Math|Transform|MakeTransform (Variables|Default|GetSpawn%20Transform%20Location_21) "0,90.000000, 0" "1,1,1") "Undefined" 0 0)
                          (Math|Integer|IncrementInt (Variables|/Game/Evolve/Core/GameMode/BP_GameMode.BP_GameMode_C|GetNbEnnemies (Variables|Default|GetBP_GameMode))
                            (:%20%20
                              (Game|SpawnActorfromClass (Variables|Default|GetEnemy4) (Math|Transform|MakeTransform (Variables|Default|GetSpawn%20Transform%20Location_22) "0,90.000000, 0" "1,1,1") "Undefined" 0 0)
                              (Math|Integer|IncrementInt (Variables|/Game/Evolve/Core/GameMode/BP_GameMode.BP_GameMode_C|GetNbEnnemies (Variables|Default|GetBP_GameMode))
                                (:%20%20
                                  (Game|SpawnActorfromClass (Variables|Default|GetEnemy5) (Math|Transform|MakeTransform (Variables|Default|GetSpawn%20Transform%20Location_23) "0,90.000000, 0" "1,1,1") "Undefined" 0 0)
                                  (Math|Integer|IncrementInt (Variables|/Game/Evolve/Core/GameMode/BP_GameMode.BP_GameMode_C|GetNbEnnemies (Variables|Default|GetBP_GameMode))
                                    (:%20%20
                                      (Game|SpawnActorfromClass (Variables|Default|GetEnemy6) (Math|Transform|MakeTransform (Variables|Default|GetSpawn%20Transform%20Location_24) "0,90.000000, 0" "1,1,1") "Undefined" 0 0)
                                      (Math|Integer|IncrementInt (Variables|/Game/Evolve/Core/GameMode/BP_GameMode.BP_GameMode_C|GetNbEnnemies (Variables|Default|GetBP_GameMode))
                                        (:%20%20
                                          (bind _result_6 (Math|Integer|DecrementInt (Variables|Default|GetNbEnemiesCurrent))
                                            (:%20%20
                                              (if (<= _result_6 0)
                                                (Utilities|Time|ClearandInvalidateTimerbyHandle (Variables|Default|GetHandleTimer))
                                                (Class|BPIMPGameMode|StopCylindre(Message) _bp_gamemode_12)
                                                (Default|IasMoves _bp_gamemode_12)))))))))))))))))))))))))

(event Custom|RemoveAffichageVageNb
  (Widget|RemovefromParent (Variables|Default|GetWidgetRef)))

(event EventBeginPlay)

(fn ConstructionScript)

(fn Win
  (if (not (Game|IsGamePaused))
    (Game|SetGamePaused true)
    (bind _returnvalue (UserInterface|CreateWidget "/Game/Base/UI/UI_Win.UI_Win_C"))
    (bind _output_get (Variables|Default|SetUI_Win _returnvalue))
    (UserInterface|Viewport|AddtoViewport _output_get 0)
    (Variables|/Script/Engine.PlayerController|SetbShowMouseCursor (Game|GetPlayerController 0) true)))