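; BP_Spowner is an enemy spawner actor that spawns a single actor of its Enemy class when play begins.
; BeginPlay calls SpawnOneEnemy, which spawns at the spawner's own transform and ignores the enemy count it receives.
; The delayed respawn call and the random point-in-box lookup are disconnected, so no repeated or area-randomized spawning occurs, despite the event's comment describing a random position.
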(event Custom|SpawnOneEnemy
  (params (Enemy :type Actor%20Class%20Reference) (SpawnTransform :type Transform) (Number%20Of%20Ennemies :type Integer))
  ;[1 1 1] Prend une position aléaqtoire dans la zone et fait apparaitre un ennemi
  (Game|SpawnActorfromClass Enemy SpawnTransform "Undefined" 0 0))

(event EventBeginPlay
  (CallFunction|SpawnOneEnemy (Variables|Default|GetEnemy) (Transformation|GetActorTransform) (Variables|Default|GetNumber%20Of%20Ennemies)))

(fn ConstructionScript)