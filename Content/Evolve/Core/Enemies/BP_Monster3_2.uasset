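; Monster enemy that fires projectiles on a looping timer from BeginPlay and takes point damage from the player.
; Its height at spawn picks one of two muzzle transforms, and each shot plays audio and Niagara cues before spawning BP_ProjectileEnemies.
; Physical surface type separates body hits from double-damage weak-spot hits, both boosted by the GameMode's weapon bonus.
; At zero health it cries out, ragdolls, reports the kill to BP_GameMode and destroys itself.
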(event Custom|Fire
  (if (> (.z (Transformation|GetActorLocation self)) 5.5e+02)
    (Variables|Default|SetAngleDeTire (Transformation|GetWorldTransform (Variables|Default|GetProjectileSpawnPoint1)))
    (else
      (Variables|Default|SetAngleDeTire (Transformation|GetWorldTransform (Variables|Default|GetProjectileSpawnPoint))))))

(event Custom|Ragdoll
  (Physics|SetSimulatePhysics (Variables|Character|GetMesh) true)
  (Pawn|Components|CharacterMovement|DisableMovement (Variables|Character|GetCharacterMovement)))

(event Custom|StopFire
  (Utilities|Time|ClearandInvalidateTimerbyHandle (Variables|Default|GetHandleTimer)))

(event Custom|UpdateisDead
  ;[1 1 1] Vérifier si le personnage est mort
  (if (<= (Variables|Default|GetPointsDeVie) 0.0)
    (Variables|Default|SetisDead? true)
    (Utilities|FlowControl|DoOnce false
      (:Completed
        (Audio|SpawnSoundAttached "/Game/Evolve/Art/Audios/CrisAlternatifs/Evolve_FX_-_Ennemis_Cris_3_Cue.Evolve_FX_-_Ennemis_Cris_3_Cue" (Variables|Collision|GetCapsuleComponent) "None" (.location (Transformation|GetWorldTransform (Variables|Default|GetProjectileSpawnPoint))) "0, 0, 0" "KeepWorldPosition" false 5e+01 1.0 0.0 0 0)))
    (else
      (Variables|Default|SetisDead? false))))

(event Custom|FireProjectile
  ;[1 1 1] Fait Apparaitre un projectile au ProjectileSpawn
  (Utilities|FlowControl|Delay 0.5)
  (bind _output_get (Variables|Default|SetPos (Math|Random|RandomInteger 2)))
  (if (== _output_get 0)
    (AddComponent|AddAudioComponent false)
    (elif (== _output_get 1)
      (AddComponent|AddAudioComponent false)
      (else
        (AddComponent|AddAudioComponent false))))
  (Utilities|FlowControl|Delay 0.5)
  (Niagara|SpawnSystemAttached "/Game/Evolve/Art/FX/Alien_Shoot/NS_AlienShoot_Projectile.NS_AlienShoot_Projectile" (Variables|Default|GetProjectileSpawnPoint) "None" (.location (Variables|Default|GetAngleDeTire)) "0, 0, 0" "KeepWorldPosition" false)
  (Utilities|FlowControl|Delay 0.25)
  (Game|SpawnActorfromClass "/Game/Evolve/Core/Enemies/BP_ProjectileEnemies.BP_ProjectileEnemies_C" (Variables|Default|GetAngleDeTire) "Undefined" 0 0))

(event Game|Damage|EventPointDamage
  (params (Damage :type Float%20%28single-precision%29) (DamageType :type Damage%20Type%20Object%20Reference) (HitLocation :type Vector :default "0, 0, 0") (HitNormal :type Vector :default "0, 0, 0") (HitComponent :type Primitive%20Component%20Object%20Reference) (BoneName :type Name :default "None") (ShotFromDirection :type Vector :default "0, 0, 0") (InstigatedBy :type Controller%20Object%20Reference) (DamageCauser :type Actor%20Object%20Reference) (HitInfo :type Hit%20Result%20Structure%20%28by%20ref%29))
  (bind _returnvalue (* Damage -1.0))
  (bind _bp_gamemode (Variables|Default|GetBP_GameMode))
  (bind _bp_gamemode_2 (Variables|Default|GetBP_GameMode))
  (bind _augmentationdégatsarme (Variables|/Game/Evolve/Core/GameMode/BP_GameMode.BP_GameMode_C|GetAugmentationDégatsArme _bp_gamemode_2))
  (bind _augmentationdégatsarme_2 (Variables|/Game/Evolve/Core/GameMode/BP_GameMode.BP_GameMode_C|GetAugmentationDégatsArme _bp_gamemode))
  (bind _returnvalue_2 (- _returnvalue _augmentationdégatsarme))
  (bind _returnvalue_3 (+ Damage _augmentationdégatsarme_2))
  (bind _returnvalue_4 (* _returnvalue_3 -2.0))
  ;[1 1 1] Gestion des dégats fait par le joueur
  (switch Utilities|FlowControl|Switch|SwitchonEPhysicalSurface (Variables|/Script/PhysicsCore.PhysicalMaterial|GetSurfaceType (.PhysMat (Collision|BreakHitResult HitInfo)))
    (:SurfaceType_Default
      (Development|PrintString (Utilities|String|Append "Body Shot" (Utilities|String|ToString(Float) _returnvalue_2)) true true "(R=0.000000,G=0.660000,B=1.000000,A=1.000000)" 1.0 :!label _label)
      (CallFunction|UpDatePV _returnvalue_2))
    (:SurfaceType1
      (Development|PrintString (Utilities|String|Append "Head Shot" (Utilities|String|ToString(Float) _returnvalue_4)) true true "(R=1.000000,G=0.054822,B=0.000000,A=1.000000)" 1.0)
      (CallFunction|UpDatePV _returnvalue_4))
    (:SurfaceType2
      (goto _label)))
  (if (Variables|Default|GetisDead?)
    (Utilities|FlowControl|DoOnce false
      (:Completed
        (AddComponent|AddAudioComponent false)
        (CallFunction|Ragdoll)
        (Utilities|FlowControl|Delay 1.5)
        (Default|KillEnemies (Variables|Default|GetBP_GameMode))
        (Actor|DestroyActor)))))

(event EventBeginPlay
  ;[1 1 1] Tire projectiles de manière répété
  (Utilities|FlowControl|Delay 0.25)
  (CallFunction|Fire)
  (bind _asbp_game_mode (Utilities|Casting|CastToBP_GameMode (Game|GetGameMode)))
  (Variables|Default|SetBP_GameMode _asbp_game_mode)
  (CallFunction|FireProjectile)
  (bind _returnvalue (Utilities|Time|SetTimerbyFunctionName 0 "FireProjectile" (/ 1.0 (Variables|Default|GetProjectilesPerSecond)) true))
  (Variables|Default|SetHandleTimer _returnvalue))

(fn ConstructionScript)

(fn UpDatePV
  (params (Delta :type Float%20%28single-precision%29))
  ;[1 1 1] Gestion PVs
  (bind _output_get (Variables|Default|SetPointsDeVie (+ Delta (Variables|Default|GetPointsDeVie))))
  (CallFunction|UpdateisDead)
  (return _output_get))