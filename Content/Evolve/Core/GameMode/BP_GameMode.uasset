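; Game mode that tracks score, living enemies and game flow, and owns the in-game HUD created at BeginPlay.
; Score increments update the HUD and open the upgrade window (Améliorations) at fixed thresholds, while the enemy countdown reaching zero asks BPSpawner for another wave.
; Améliorations toggles pause, widget and mouse cursor together; Win, not called within this Blueprint, pauses and shows the victory screen.
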(event Custom|KillEnemies
  (bind _result (Math|Integer|DecrementInt (Variables|Default|GetNbEnnemies))
    (:%20%20
      (if (== _result 0)
        (Default|WaveSpawn (Variables|Default|GetBP_Spawner))))))

(event EventBeginPlay
  (bind _returnvalue (UserInterface|CreateWidget "/Game/Evolve/UI/UI_IngameHUD.UI_IngameHUD_C"))
  (bind _output_get (Variables|Default|SetUI_HUD _returnvalue))
  (UserInterface|Viewport|AddtoViewport _output_get 0))

(event EventUpdateUIPlayerScore1
  (bind _result (Math|Integer|IncrementInt (Variables|Default|GetCurrent%20Score))
    (:%20%20
      (Default|UpdateScore (Variables|Default|GetUI_HUD) _result)
      (if (== _result 3)
        (CallFunction|Améliorations)
        (elif (== _result 11)
          (CallFunction|Améliorations)
          (elif (== _result 21)
            (CallFunction|Améliorations)
            (elif (== _result 36)
              (CallFunction|Améliorations))))))))

(fn ConstructionScript)

(fn Win
  (if (not (Game|IsGamePaused))
    (Game|SetGamePaused true)
    (bind _returnvalue (UserInterface|CreateWidget "/Game/Base/UI/UI_Win.UI_Win_C"))
    (bind _output_get (Variables|Default|SetUI_Win _returnvalue))
    (UserInterface|Viewport|AddtoViewport _output_get 0)
    (Variables|/Script/Engine.PlayerController|SetbShowMouseCursor (Game|GetPlayerController 0) true)))

(fn Améliorations
  (if (Game|IsGamePaused)
    (Game|SetGamePaused false)
    (Widget|RemovefromParent (Variables|Default|GetUI_FenètreAméliorations))
    (Variables|/Script/Engine.PlayerController|SetbShowMouseCursor (Game|GetPlayerController 0) false)
    (else
      (Game|SetGamePaused true)
      (bind _returnvalue (UserInterface|CreateWidget "/Game/Evolve/UI/UI_FenètreAméliorations.UI_FenètreAméliorations_C"))
      (bind _output_get (Variables|Default|SetUI_FenètreAméliorations _returnvalue))
      (UserInterface|Viewport|AddtoViewport _output_get 0)
      (Variables|/Script/Engine.PlayerController|SetbShowMouseCursor (Game|GetPlayerController 0) true))))