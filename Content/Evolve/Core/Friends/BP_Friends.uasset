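; Friendly character Blueprint that auto-fires its gun on a looping FireRate timer and has health, destroying itself when dead.
; Point damage reads the hit's physical surface, doubling damage on Weak Spot, and prints debug text.
; A player entering its box starts an uncleared looping timer that repeatedly sends a positive health change to AsEnnemi, which is never set here.
; A BodyColor function, uncalled here, tints the armor red through a dynamic material.
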(event OnComponentBeginOverlap(Box)
  (params (OverlappedComponent :type Primitive%20Component%20Object%20Reference) (OtherActor :type Actor%20Object%20Reference) (OtherComp :type Primitive%20Component%20Object%20Reference) (OtherBodyIndex :type Integer) (bFromSweep :type Boolean) (SweepResult :type Hit%20Result%20Structure%20%28by%20ref%29))
  (bind _asbp_player (Utilities|Casting|CastToBP_Player OtherActor))
  (Variables|Default|SetAs%20BP%20Player _asbp_player)
  (CallFunction|DamageH)
  (Utilities|Time|SetTimerbyEvent (delegate Custom|DamageH) (/ 1.0 3.0) true))

(event Custom|DamageH
  (Class|BPIDommages|AffectPV(Message) (Variables|Default|GetAs%20Ennemi) 5.0))

(event Custom|EnemyFire
  ;[1 1 1] Permet de tirer
  (Default|FireGun (Variables|Default|GetGun)))

(event Custom|AffectPV_1
  (params (Delta :type Float%20%28single-precision%29))
  ;[1 1 1] Gestion des dégats
  (bind _newpv (CallFunction|UpDatePV Delta))
  (Development|PrintString (Utilities|String|ToString(Float) _newpv))
  (if (Variables|Default|GetisDead?)
    (Actor|DestroyActor)))

(event Game|Damage|EventPointDamage
  (params (Damage :type Float%20%28single-precision%29) (DamageType :type Damage%20Type%20Object%20Reference) (HitLocation :type Vector :default "0, 0, 0") (HitNormal :type Vector :default "0, 0, 0") (HitComponent :type Primitive%20Component%20Object%20Reference) (BoneName :type Name :default "None") (ShotFromDirection :type Vector :default "0, 0, 0") (InstigatedBy :type Controller%20Object%20Reference) (DamageCauser :type Actor%20Object%20Reference) (HitInfo :type Hit%20Result%20Structure%20%28by%20ref%29))
  (switch Utilities|FlowControl|Switch|SwitchonEPhysicalSurface (Variables|/Script/PhysicsCore.PhysicalMaterial|GetSurfaceType (.PhysMat (Collision|BreakHitResult HitInfo)))
    (:SurfaceType_Default
      (Development|PrintString (Utilities|String|Append "Body Shot" (Utilities|String|ToString(Float) Damage)) true true "(R=0.000000,G=0.660000,B=1.000000,A=1.000000)" 5.0 :!label _label)
      ;[1 1 1] Gestion des dégats
      (bind _newpv (CallFunction|UpDatePV (* Damage -1.0)))
      (Development|PrintString (Utilities|String|Append "" (Utilities|String|ToString(Float) _newpv)))
      (if (Variables|Default|GetisDead?)
        (Actor|DestroyActor)
        (Development|PrintString "")))
    (:SurfaceType1
      (Development|PrintString (Utilities|String|Append "Head Shot" (Utilities|String|ToString(Float) (* Damage 2.0))) true true "(R=0.244792,G=0.034765,B=0.022583,A=1.000000)" 5.0)
      ;[1 1 1] Gestion des dégats
      (bind _newpv_2 (CallFunction|UpDatePV (* Damage -2.0)))
      (Development|PrintString (Utilities|String|Append "" (Utilities|String|ToString(Float) _newpv_2)))
      (if (Variables|Default|GetisDead?)
        (Actor|DestroyActor)
        (Development|PrintString "")))
    (:SurfaceType2
      (goto _label))))

(event EventBeginPlay
  ;[1 1 1] Permet de tirer
  (Utilities|Time|SetTimerbyEvent (delegate Custom|EnemyFire) (Variables|Default|GetFireRate) true))

(fn ConstructionScript
  (|CallParentFunction))

(fn BodyColor
  (bind _returnvalue (Rendering|Material|CreateDynamicMaterialInstance (Variables|Character|GetMesh) 3 0 "None" :!class /Script/Engine.PrimitiveComponent))
  (bind _output_get (Variables|Default|SetBody%20Materiel _returnvalue))
  (Rendering|Material|SetVectorParameterValue _output_get "PrimaryArmorColor" "(R=0.863157,G=0.043735,B=0.042311,A=1.000000)" :!class /Script/Engine.MaterialInstanceDynamic))