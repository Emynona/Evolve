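; BP_PointLight5 is a point light that goes dark for a delay when the game's current wave number differs from its own counter.
; On BeginPlay it waits, turns the light on, then starts a looping timer that polls BP_GameMode's NbWaveCurrent.
; On each mismatch it decrements Compteur and hides the light, restoring visibility after the same Delay variable.
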(event Custom|Lumières
  (bind _asbp_game_mode (Utilities|Casting|CastToBP_GameMode (Game|GetGameMode)))
  (bind _output_get (Variables|Default|SetAs%20BP%20Game%20Mode _asbp_game_mode))
  (if (!= (Variables|/Game/Evolve/Core/GameMode/BP_GameMode.BP_GameMode_C|GetNbWaveCurrent _output_get) (Variables|Default|GetCompteur))
    (Math|Integer|DecrementInt (Variables|Default|GetCompteur)
      (:%20%20
        (Rendering|SetVisibility (Variables|Default|GetLightComponent) false false)
        (Utilities|FlowControl|Delay (Variables|Default|GetDelay))
        (Rendering|SetVisibility (Variables|Default|GetLightComponent) true false)))))

(event EventBeginPlay
  (Utilities|FlowControl|Delay (Variables|Default|GetDelay))
  (Rendering|SetVisibility (Variables|Default|GetLightComponent) true false)
  (Utilities|Time|SetTimerbyFunctionName 0 "Lumières" 0.1 true))

(fn ConstructionScript)