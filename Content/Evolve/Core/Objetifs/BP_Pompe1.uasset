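; BP_Pompe1 is a destructible pump objective with hit points that upgrades can raise through the game mode's bonus value.
; AffectHP applies a delta, sends normalized HP to the game mode's UI and checks for death.
; On destruction it decrements the pump count, clears the Pompe01 flag, destroys itself and signals six AI move messages.
; Older tiered-upgrade logic and coolant projectile spawning remain unconnected.
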(event Custom|UpdateisDead
  ;[1 1 1] Vérifier si le personnage est mort
  (if (<= (Variables|Default|GetPoints%20De%20Vie) 0.0)
    (Variables|Default|SetIs%20Dead? true)
    (else
      (Variables|Default|SetIs%20Dead? false))))

(event Custom|UpdatePompesAméliorations
  (Variables|Default|SetPoints%20De%20Vie (+ (Variables|/Game/Evolve/Core/GameMode/BP_GameMode.BP_GameMode_C|GetAugmentationPVsPompes (Variables|Default|GetAs%20BP%20Game%20Mode)) (Variables|Default|GetPoints%20De%20Vie))))

(event EventAffectHP
  (params (Delta :type Float%20%28single-precision%29))
  (bind _as_bp_game_mode (Variables|Default|GetAs%20BP%20Game%20Mode))
  ;[1 1 1] Gestion des dégats
  (bind _newpv (CallFunction|UpDatePV Delta))
  (Class|BPIGameMode|UPdateUIPlayerHP(Message) (Game|GetGameMode) (CallFunction|GetNormalLifeHP))
  (Development|PrintString (Utilities|String|Append "PVs pompe 1 restant: " (Utilities|String|ToString(Float) _newpv)) true true "(R=1.000000,G=0.358212,B=0.498699,A=1.000000)" 1.0)
  (if (Variables|Default|GetIs%20Dead?)
    (Development|PrintString "Pompe détruit" true true "(R=0.583333,G=0.046313,B=0.000000,A=1.000000)" 6e+01)
    (bind _asbp_game_mode (Utilities|Casting|CastToBP_GameMode (Game|GetGameMode)))
    (Math|Integer|DecrementInt (Variables|/Game/Evolve/Core/GameMode/BP_GameMode.BP_GameMode_C|GetNbrPompes _asbp_game_mode)
      (:%20%20
        (Variables|/Game/Evolve/Core/GameMode/BP_GameMode.BP_GameMode_C|SetPompe01 _asbp_game_mode false)
        (Actor|DestroyActor)
        (Class|BPIMPGameMode|IA1Move(Message) _as_bp_game_mode)
        (Class|BPIMPGameMode|IA2Move(Message) _as_bp_game_mode)
        (Class|BPIMPGameMode|IA3Move(Message) _as_bp_game_mode)
        (Class|BPIMPGameMode|IA4Move(Message) _as_bp_game_mode)
        (Class|BPIMPGameMode|IA5Move(Message) _as_bp_game_mode)
        (Class|BPIMPGameMode|IA6Move(Message) _as_bp_game_mode)))))

(event EventBeginPlay
  ;[1 1 1] Tire projectiles de manière répété
  (bind _asbp_game_mode (Utilities|Casting|CastToBP_GameMode (Game|GetGameMode)))
  (Variables|Default|SetAs%20BP%20Game%20Mode _asbp_game_mode))

(fn ConstructionScript)

(fn UpDatePV
  (params (delta :type Float%20%28single-precision%29))
  ;[1 1 1] Gestion PVs
  (bind _output_get (Variables|Default|SetPoints%20De%20Vie (+ delta (Variables|Default|GetPoints%20De%20Vie))))
  (CallFunction|UpdateisDead)
  (return _output_get))

(fn GetNormalLifeHP
  ;[1 1 1] Récupère les pvs du joueur sur un échelle de 0 à 1
  (return (/ (Variables|Default|GetPoints%20De%20Vie) (Variables|Default|GetMaxPointsDeVie))))