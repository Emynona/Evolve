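; Reactor objective actor that triggers the game's defeat once no pumps remain.
; A looping Surchauffe timer polls NbrPompes on BP_GameMode, then destroys the reactor and calls Lose.
; Lose pauses the game and shows the defeat widget with the mouse cursor; Win mirrors it but is not called here.
; Hit-point helpers remain, but their overheating drain and death checks are disconnected, and UpdateisDead is empty.
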(event Custom|UpdateisDead
  ;[1 1 1] Vérifier si le personnage est mort
)

(event Custom|Surchauffe
  ;[1 1 1] Quantité de point de vie que le réacteur perd par seconde + Conditions de victoires/défaites
  (bind _asbp_game_mode (Utilities|Casting|CastToBP_GameMode (Game|GetGameMode)))
  (if (<= (Variables|/Game/Evolve/Core/GameMode/BP_GameMode.BP_GameMode_C|GetNbrPompes _asbp_game_mode) 0)
    (Development|PrintString "Réacteur Détruit" true true "(R=0.307292,G=0.000000,B=0.147192,A=1.000000)" 1e+01)
    (Actor|DestroyActor)
    (CallFunction|Lose)))

(event EventBeginPlay
  ;[1 1 1] Combien de fois le réacteur perd des points de vie toutes les secondes
  (Utilities|Time|SetTimerbyFunctionName 0 "Surchauffe" 0.1 true))

(event EventBonusPV
  (params (Delta :type Float%20%28single-precision%29))
  ;[1 1 1] Gestion des dégats
)

(fn ConstructionScript)

(fn UpDatePVs
  (params (Delta :type Float%20%28single-precision%29))
  ;[1 1 1] Gestion PVs
  (bind _output_get (Variables|Default|SetPointsDeVie (+ Delta (Variables|Default|GetPointsDeVie))))
  (CallFunction|UpdateisDead)
  (return _output_get))

(fn CompteurPVs
  (params (Delta :type Float%20%28single-precision%29))
  ;[1 1 1] Gestion PVs
  (bind _output_get (Variables|Default|SetComptPVs (+ Delta (Variables|Default|GetComptPVs))))
  (CallFunction|UpdateisDead)
  (return _output_get))

(fn Lose
  (if (not (Game|IsGamePaused))
    (Game|SetGamePaused true)
    (bind _returnvalue (UserInterface|CreateWidget "/Game/Base/UI/UI_Lose.UI_Lose_C"))
    (bind _output_get (Variables|Default|SetUI_Lose _returnvalue))
    (UserInterface|Viewport|AddtoViewport _output_get 0)
    (Variables|/Script/Engine.PlayerController|SetbShowMouseCursor (Game|GetPlayerController 0) true)))

(fn Win
  (if (not (Game|IsGamePaused))
    (Game|SetGamePaused true)
    (bind _returnvalue (UserInterface|CreateWidget "/Game/Base/UI/UI_Win.UI_Win_C"))
    (bind _output_get (Variables|Default|SetUI_Win _returnvalue))
    (UserInterface|Viewport|AddtoViewport _output_get 0)
    (Variables|/Script/Engine.PlayerController|SetbShowMouseCursor (Game|GetPlayerController 0) true)))

(fn GetNormalLifeHP
  ;[1 1 1] Récupère les pvs du joueur sur un échelle de 0 à 1
  (return (/ (Variables|Default|GetPointsDeVie) (Variables|Default|GetMaxPointsDeVie))))