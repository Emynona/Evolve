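; BP_Pompe3 is the third pump objective, a destructible actor with hit points.
; AffectHP applies a signed delta through UpDatePV, which refreshes IsDead, and prints the remaining health.
; On death it decrements the GameMode's pump count, clears its Pompe03 flag and destroys itself.
; FireProjectile can spawn coolant (BP_LiquideDeRefroidisement) at LaserToReact, but the repeating timer meant to call it is disconnected from BeginPlay.
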(event Custom|UpdateisDead
  ;[1 1 1] Vérifier si le personnage est mort
  (if (<= (Variables|Default|GetPoints%20De%20Vie) 0.0)
    (Variables|Default|SetIs%20Dead? true)
    (else
      (Variables|Default|SetIs%20Dead? false))))

(event Custom|FireProjectile
  ;[1 1 1] Fait Apparaitre un projectile au ProjectileSpawn
  (Game|SpawnActorfromClass "/Game/Evolve/Core/Objetifs/BP_LiquideDeRefroidisement.BP_LiquideDeRefroidisement_C" (Transformation|GetWorldTransform (Variables|Default|GetLaserToReact)) "Undefined" 0 0))

(event EventAffectHP
  (params (Delta :type Float%20%28single-precision%29))
  ;[1 1 1] Gestion des dégats
  (bind _newpv (CallFunction|UpDatePV Delta))
  (Development|PrintString (Utilities|String|Append "PVs pompe restant: " (Utilities|String|ToString(Float) _newpv)) true true "(R=1.000000,G=0.358212,B=0.498699,A=1.000000)" 0.5)
  (if (Variables|Default|GetIs%20Dead?)
    (Development|PrintString "Pompe détruit" true true "(R=0.583333,G=0.046313,B=0.000000,A=1.000000)" 1.2e+02)
    (bind _asbp_game_mode (Utilities|Casting|CastToBP_GameMode (Game|GetGameMode)))
    (Math|Integer|DecrementInt (Variables|/Game/Evolve/Core/GameMode/BP_GameMode.BP_GameMode_C|GetNbrPompes _asbp_game_mode)
      (:%20%20
        (Variables|/Game/Evolve/Core/GameMode/BP_GameMode.BP_GameMode_C|SetPompe03 _asbp_game_mode false)
        (Actor|DestroyActor)))))

(event EventBeginPlay
  ;[1 1 1] Tire projectiles de manière répété
)

(fn ConstructionScript)

(fn UpDatePV
  (params (delta :type Float%20%28single-precision%29))
  ;[1 1 1] Gestion PVs
  (bind _output_get (Variables|Default|SetPoints%20De%20Vie (+ delta (Variables|Default|GetPoints%20De%20Vie))))
  (CallFunction|UpdateisDead)
  (return _output_get))