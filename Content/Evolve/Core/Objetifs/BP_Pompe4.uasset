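; BP_Pompe4 is the fourth pump objective, with health that can be damaged or upgraded.
; Each HP change passes the normalized health to the first BP_Pumps03 found, updating its water level, plus damage effects on hits.
; At zero HP it triggers that actor's destruction, updates BP_GameMode pump state and score, calls IAsMoves and destroys itself.
; The coolant projectile spawn never runs.
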(event Custom|UpdateisDead
  ;[1 1 1] Vérifier si le personnage est mort
  (if (<= (Variables|Default|GetPoints%20De%20Vie) 0.0)
    (Variables|Default|SetIs%20Dead? true)
    (else
      (Variables|Default|SetIs%20Dead? false))))

(event Custom|Augmentation
  ;[1 1 1] Permt l'amélioration des PVs
  (Variables|Default|SetMaxPointsDeVie (+ (Variables|Default|GetMaxPointsDeVie) 2.5e+02))
  (CallFunction|UpDatePV (Variables|/Game/Evolve/Core/GameMode/BP_GameMode.BP_GameMode_C|GetAugmentationPVsPompes (Variables|Default|GetAs%20BP%20Game%20Mode)))
  (bind _outactors (Actor|GetAllActorsOfClass "/Game/Evolve/Art/Blueprints/BP_Pumps03.BP_Pumps03_C"))
  (Variables|/Game/Evolve/Art/Blueprints/BP_Pumps03.BP_Pumps03_C|SetFillLevel (Utilities|Array|Get(acopy) _outactors) (CallFunction|GetNormalLifeHP))
  (Default|WaterLevel (Utilities|Array|Get(acopy) _outactors)))

(event EventAffectHP
  (params (Delta :type Float%20%28single-precision%29))
  (bind _as_bp_game_mode (Variables|Default|GetAs%20BP%20Game%20Mode))
  ;[1 1 1] Gestion des dégats
  (CallFunction|UpDatePV Delta)
  (bind _outactors (Actor|GetAllActorsOfClass "/Game/Evolve/Art/Blueprints/BP_Pumps03.BP_Pumps03_C"))
  (Variables|/Game/Evolve/Art/Blueprints/BP_Pumps03.BP_Pumps03_C|SetFillLevel (Utilities|Array|Get(acopy) _outactors) (CallFunction|GetNormalLifeHP))
  (Default|Dégats (Utilities|Array|Get(acopy) _outactors))
  (Default|WaterLevel (Utilities|Array|Get(acopy) _outactors))
  (if (Variables|Default|GetIs%20Dead?)
    (Default|Destruction (Utilities|Array|Get(acopy) _outactors))
    (bind _asbp_game_mode (Utilities|Casting|CastToBP_GameMode (Game|GetGameMode)))
    (Math|Integer|DecrementInt (Variables|/Game/Evolve/Core/GameMode/BP_GameMode.BP_GameMode_C|GetNbrPompes _asbp_game_mode)
      (:%20%20
        (Variables|/Game/Evolve/Core/GameMode/BP_GameMode.BP_GameMode_C|SetPompe04 _asbp_game_mode false)
        (Actor|DestroyActor)
        (Default|IasMoves _as_bp_game_mode)
        (Variables|/Game/Evolve/Core/GameMode/BP_GameMode.BP_GameMode_C|SetCurrent%20Score _as_bp_game_mode (- (Variables|/Game/Evolve/Core/GameMode/BP_GameMode.BP_GameMode_C|GetCurrent%20Score _as_bp_game_mode) 10))
        (Math|Integer|DecrementInt (Variables|/Game/Evolve/Core/GameMode/BP_GameMode.BP_GameMode_C|GetNbrPompesRestantes _as_bp_game_mode))))))

(event EventBeginPlay
  ;[1 1 1] Tire projectiles de manière répété
  (bind _asbp_game_mode (Utilities|Casting|CastToBP_GameMode (Game|GetGameMode)))
  (Variables|Default|SetAs%20BP%20Game%20Mode _asbp_game_mode))

(fn ConstructionScript)

(fn UpDatePV
  (params (delta :type Float%20%28single-precision%29))
  ;[1 1 1] Gestion PVs
  (bind _output_get (Variables|Default|SetPoints%20De%20Vie (+ delta (Variables|Default|GetPoints%20De%20Vie))))
  (CallFunction|UpdateisDead)
  (return _output_get))

(fn GetNormalLifeHP
  ;[1 1 1] Récupère les pvs du joueur sur un échelle de 0 à 1
  (return (/ (Variables|Default|GetPoints%20De%20Vie) (Variables|Default|GetMaxPointsDeVie))))