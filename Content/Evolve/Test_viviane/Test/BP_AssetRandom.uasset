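; BP_AssetRandom is a test actor Blueprint that dresses itself with randomly chosen static meshes.
; Its construction script applies an exposed or stored transform to ObjectOrigin, then gives the Table and Table1 components independent random picks from the first four MeshLibrary01 entries.
; The picks use an unseeded random integer, so meshes can change whenever construction reruns; the event graph has no active logic.
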(event EventBeginPlay)

(event Collision|EventActorBeginOverlap
  (params (OtherActor :type Actor%20Object%20Reference)))

(event EventTick
  (params (DeltaSeconds :type Float%20%28single-precision%29)))

(fn ConstructionScript
  (Transformation|SetRelativeTransform (Variables|Default|GetobjectOrigin) (Variables|Default|GetObjectOrigin_Tranform) false false)
  (Components|StaticMesh|SetStaticMesh (Variables|Default|Gettable) (Utilities|Array|Get(acopy) (Variables|Default|GetMeshLibrary_01) (Math|Random|RandomIntegerinRange 0 3)))
  (Components|StaticMesh|SetStaticMesh (Variables|Default|Gettable1) (Utilities|Array|Get(acopy) (Variables|Default|GetMeshLibrary_01) (Math|Random|RandomIntegerinRange 0 3))))